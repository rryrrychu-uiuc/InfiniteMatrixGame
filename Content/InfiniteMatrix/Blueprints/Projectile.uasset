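; Projectile actor that flies forward at a speed based on the player's and awards score through its Parent reference.
; SetSpeed adds a fixed boost to the given player speed and applies it to the projectile movement component along local X.
; DestroyEnemy increases the Parent's score, refreshes its score UI, destroys the projectile itself and plays a 2D sound.
; Event graph and construction script are empty, so both functions rely on external callers.
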(fn `DestroyEnemy`
  (bind _parent (`self.Parent`))
  (bind _score (`/Game/InfiniteMatrix/Blueprints/BP_Player.UpdateScore` _parent true false))
  (`/Game/InfiniteMatrix/UI/DisplayScore.UpdateScoreDisplay` (`/Game/InfiniteMatrix/Blueprints/BP_Player.ScoreUI` _parent) _score)
  (`self.K2_DestroyActor`)
  (`GameplayStatics.PlaySound2D` "/Game/InfiniteMatrix/Audio/super-mario-64-yahoo-sound_Cue.super-mario-64-yahoo-sound_Cue" 1.0 1.0 0.0 null null))

(fn `SetSpeed`
  (params (PlayerSpeed :type "Float (double-precision)"))
  (bind _returnvalue (+ PlayerSpeed 5000.0))
  (set `ProjectileMovementComponent.InitialSpeed` _returnvalue (`self.ProjectileMovement`))
  (`ProjectileMovementComponent.SetVelocityInLocalSpace` (`self.ProjectileMovement`) (`KismetMathLibrary.MakeVector` _returnvalue)))

(fn `UserConstructionScript`)