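; BP_Tunnel is a tunnel segment for an endless runner, with a rotating holed wall, an enemy and a health pack.
; Its trigger asks TunnelSpawner for another segment, destroys this one and raises player score and speed.
; Hazard hits cut health and speed and can end the run; projectiles destroy enemies but die on walls.
; Uncalled here, helper functions randomize wall shape, pickup presence and enemy position, moving one mesh rather than spawning enemies.
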(event `self.TriggerZone.OnComponentBeginOverlap`
  (params (OverlappedComponent :type "PrimitiveComponent Object Reference") (OtherActor :type "Actor Object Reference") (OtherComp :type "PrimitiveComponent Object Reference") (OtherBodyIndex :type Integer) (bFromSweep :type Boolean) (SweepResult :type "HitResult Structure (by ref)"))
  (bind _asbp_player (cast `/Game/InfiniteMatrix/Blueprints/BP_Player` OtherActor))
  (`/Game/InfiniteMatrix/Blueprints/BP_TunnelSpawner.SpawnTunnelAtSpawnPoint` (`self.TunnelSpawner`))
  (`self.K2_DestroyActor`)
  (bind _score (`/Game/InfiniteMatrix/Blueprints/BP_Player.UpdateScore` _asbp_player true false))
  (`/Game/InfiniteMatrix/UI/DisplayScore.UpdateScoreDisplay` (`/Game/InfiniteMatrix/Blueprints/BP_Player.ScoreUI` _asbp_player) _score)
  (`/Game/InfiniteMatrix/Blueprints/BP_Player.UpdateSpeed` _asbp_player true)
  (`self.SetLifeSpan` 10.0))

(event `self.ReceiveTick`
  (params (DeltaSeconds :type "Float (single-precision)"))
  (`SceneComponent.K2_AddLocalRotation` (`self.WallMesh`) (`KismetMathLibrary.MakeRotator` (* DeltaSeconds (`self.RotateSpeed`))) false false))

(event `self.WallMesh.OnComponentBeginOverlap`
  (params (OverlappedComponent :type "PrimitiveComponent Object Reference") (OtherActor :type "Actor Object Reference") (OtherComp :type "PrimitiveComponent Object Reference") (OtherBodyIndex :type Integer) (bFromSweep :type Boolean) (SweepResult :type "HitResult Structure (by ref)"))
  (bind _returnvalue (`GameplayStatics.GetObjectClass` OtherActor))
  (if (`KismetMathLibrary.ClassIsChildOf` _returnvalue "/Game/InfiniteMatrix/Blueprints/BP_Player.BP_Player_C")
    (bind _asbp_player (cast `/Game/InfiniteMatrix/Blueprints/BP_Player` OtherActor))
    (if (> (`/Game/InfiniteMatrix/Blueprints/BP_Player.Health` _asbp_player) 0)
      (`/Game/InfiniteMatrix/Blueprints/BP_Player.UpdateScore` _asbp_player false false)
      (`/Game/InfiniteMatrix/Blueprints/BP_Player.UpdateHealth` _asbp_player false)
      (`/Game/InfiniteMatrix/Blueprints/BP_Player.UpdateSpeed` _asbp_player false)
      (bind _healthstatus (`/Game/InfiniteMatrix/Blueprints/BP_Player.IsZeroHealth` _asbp_player))
      (if _healthstatus
        (set `/Game/InfiniteMatrix/Blueprints/BP_Player.IsDead` true _asbp_player)
        (`/Game/InfiniteMatrix/Blueprints/BP_Player.DisplayRestart` _asbp_player)))
    (elif (`KismetMathLibrary.ClassIsChildOf` _returnvalue "/Game/InfiniteMatrix/Blueprints/Projectile.Projectile_C")
      (`self.K2_DestroyActor` OtherActor))))

(event `self.HealthpackMesh.OnComponentBeginOverlap`
  (params (OverlappedComponent :type "PrimitiveComponent Object Reference") (OtherActor :type "Actor Object Reference") (OtherComp :type "PrimitiveComponent Object Reference") (OtherBodyIndex :type Integer) (bFromSweep :type Boolean) (SweepResult :type "HitResult Structure (by ref)"))
  (bind _asbp_player (cast `/Game/InfiniteMatrix/Blueprints/BP_Player` OtherActor))
  (`/Game/InfiniteMatrix/Blueprints/BP_Player.UpdateHealth` _asbp_player true)
  (`ActorComponent.K2_DestroyComponent` (`self.HealthpackMesh`)))

(event `self.EnemyMesh.OnComponentBeginOverlap`
  (params (OverlappedComponent :type "PrimitiveComponent Object Reference") (OtherActor :type "Actor Object Reference") (OtherComp :type "PrimitiveComponent Object Reference") (OtherBodyIndex :type Integer) (bFromSweep :type Boolean) (SweepResult :type "HitResult Structure (by ref)"))
  (bind _returnvalue (`GameplayStatics.GetObjectClass` OtherActor))
  (if (`KismetMathLibrary.ClassIsChildOf` _returnvalue "/Game/InfiniteMatrix/Blueprints/BP_Player.BP_Player_C")
    (bind _asbp_player (cast `/Game/InfiniteMatrix/Blueprints/BP_Player` OtherActor))
    (`/Game/InfiniteMatrix/Blueprints/BP_Player.UpdateHealth` _asbp_player false)
    (`ActorComponent.K2_DestroyComponent` (`self.EnemyMesh`))
    (`/Game/InfiniteMatrix/Blueprints/BP_Player.UpdateSpeed` _asbp_player false)
    (bind _healthstatus (`/Game/InfiniteMatrix/Blueprints/BP_Player.IsZeroHealth` _asbp_player))
    (if _healthstatus
      (set `/Game/InfiniteMatrix/Blueprints/BP_Player.IsDead` true _asbp_player)
      (`/Game/InfiniteMatrix/Blueprints/BP_Player.DisplayRestart` _asbp_player))
    (elif (`KismetMathLibrary.ClassIsChildOf` _returnvalue "/Game/InfiniteMatrix/Blueprints/Projectile.Projectile_C")
      (bind _asprojectile (cast `/Game/InfiniteMatrix/Blueprints/Projectile` OtherActor))
      (`/Game/InfiniteMatrix/Blueprints/Projectile.DestroyEnemy` _asprojectile)
      (`ActorComponent.K2_DestroyComponent` (`self.EnemyMesh`)))))

(fn `RandomizeWall`
  (bind _wallmesh (`self.WallMesh`))
  (`StaticMeshComponent.SetStaticMesh` _wallmesh (select `int` (`KismetMathLibrary.RandomIntegerInRange` 0 3) :`0` "/Game/InfiniteMatrix/Meshes/SM_Hole_01.SM_Hole_01" :`1` "/Game/InfiniteMatrix/Meshes/SM_Hole_02.SM_Hole_02" :`2` "/Game/InfiniteMatrix/Meshes/SM_Hole_03.SM_Hole_03" :`3` "/Game/InfiniteMatrix/Meshes/SM_Hole_04.SM_Hole_04" :!type "StaticMesh Object Reference"))
  (`SceneComponent.K2_AddLocalRotation` _wallmesh (`KismetMathLibrary.MakeRotator` (`KismetMathLibrary.RandomFloatInRange` 0.0 360.0)) false false))

(fn `SpawnEnemies `
  (for _ (range (+ (`KismetMathLibrary.RandomInteger` 2) 1))
    (`SceneComponent.K2_AddRelativeLocation` (`self.EnemyMesh`) (`KismetMathLibrary.MakeVector` (`KismetMathLibrary.RandomFloatInRange` -750.0 750.0) (`KismetMathLibrary.RandomFloatInRange` -300.0 300.0) (`KismetMathLibrary.RandomFloatInRange` -300.0 300.0)) false false)))

(fn `SpawnHealthPack`
  (bind _healthpackmesh (`self.HealthpackMesh`))
  (if (> (`KismetMathLibrary.RandomInteger` 9) 0)
    (`ActorComponent.K2_DestroyComponent` _healthpackmesh)
    (else
      (`SceneComponent.K2_AddRelativeLocation` _healthpackmesh (`KismetMathLibrary.MakeVector` (`KismetMathLibrary.RandomFloatInRange` -750.0 750.0) (`KismetMathLibrary.RandomFloatInRange` -300.0 300.0) (`KismetMathLibrary.RandomFloatInRange` -300.0 300.0)) false false))))

(fn `UserConstructionScript`)